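; Panel is a furniture actor that mounts onto a Wall when its Box overlaps one.
; The overlap marks the Wall used and stores it, then Tick teleports the panel to that Wall's Point transform with 90 degrees added yaw and hides ButtonRotate.
; Ending overlap with a Wall frees it and destroys the panel.
; RotateRight and RotateLeft are identical, both adding the actor's current rotation locally.
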(event OnComponentBeginOverlap(Box)
  (params (OverlappedComponent :type Primitive%20Component%20Object%20Reference) (OtherActor :type Actor%20Object%20Reference) (OtherComp :type Primitive%20Component%20Object%20Reference) (OtherBodyIndex :type Integer) (bFromSweep :type Boolean) (SweepResult :type Hit%20Result%20Structure%20%28by%20ref%29))
  (bind _aswall (Utilities|Casting|CastToWall OtherActor))
  (Variables|/Game/Blueprint/furniture/RemovableActor.RemovableActor_C|Setused? _aswall true)
  (Variables|Default|SetReferenceWall _aswall))

(event OnComponentEndOverlap(Box)
  (params (OverlappedComponent :type Primitive%20Component%20Object%20Reference) (OtherActor :type Actor%20Object%20Reference) (OtherComp :type Primitive%20Component%20Object%20Reference) (OtherBodyIndex :type Integer))
  (bind _aswall (Utilities|Casting|CastToWall OtherActor))
  (Variables|/Game/Blueprint/furniture/RemovableActor.RemovableActor_C|Setused? _aswall false)
  (Variables|Default|SetReferenceWall 0)
  (Actor|DestroyActor))

(event EventBeginPlay
  (|CallParentFunction))

(event Collision|EventActorBeginOverlap
  (params (OtherActor :type Actor%20Object%20Reference)))

(event EventTick
  (params (DeltaSeconds :type Float%20%28single-precision%29))
  (bind _referencewall (Variables|Default|GetReferenceWall))
  (bind _point (Variables|/Game/Blueprint/furniture/Wall.Wall_C|Getpoint _referencewall))
  (bind _returnvalue (Transformation|GetWorldTransform _point))
  (bind (_location _rotation) (Math|Transform|BreakTransform _returnvalue))
  (bind (_roll _pitch _yaw) (Math|Rotator|BreakRotator _rotation))
  (|CallParentFunction DeltaSeconds)
  (Utilities|IsValid _referencewall
    (:Is%20Valid
      (Transformation|SetActorTransform (Math|Transform|MakeTransform _location (Math|Rotator|MakeRotator _roll _pitch (+ _yaw 9e+01))) false true)
      (Rendering|SetVisibility (Variables|Default|GetButtonRotate) false false))))

(event EventRotateLeft
  (bind _returnvalue (Transformation|GetActorRotation))
  (Transformation|AddActorLocalRotation (Math|Rotator|MakeRotator (.roll _returnvalue) (.pitch _returnvalue) (.yaw _returnvalue)) false false))

(event EventRotateRight
  (bind _returnvalue (Transformation|GetActorRotation))
  (Transformation|AddActorLocalRotation (Math|Rotator|MakeRotator (.roll _returnvalue) (.pitch _returnvalue) (.yaw _returnvalue)) false false))

(fn ConstructionScript
  (|CallParentFunction))