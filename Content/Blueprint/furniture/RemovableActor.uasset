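; RemovableActor is a placeable furniture piece that can be selected, rotated in 90-degree steps and tinted red or blue, with opacity reflecting placement.
; Box overlaps toggle Used on GridBase cells and, for non-floor pieces, other RemovableActors; non-floor pieces self-destroy on other overlaps.
; Selection spawns a duplicate outline mesh, synced on Tick, and shows the rotate widget for non-floor pieces.
; Label and rotate widgets receive a self-reference on BeginPlay.
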(event OnComponentBeginOverlap(Box)
  (params (OverlappedComponent :type Primitive%20Component%20Object%20Reference) (OtherActor :type Actor%20Object%20Reference) (OtherComp :type Primitive%20Component%20Object%20Reference) (OtherBodyIndex :type Integer) (bFromSweep :type Boolean) (SweepResult :type Hit%20Result%20Structure%20%28by%20ref%29))
  (bind _asgrid_base (Utilities|Casting|CastToGridBase OtherActor)
    (:then
      (if (not (Variables|/Game/Blueprint/Grid/GridBase.GridBase_C|GetUsed _asgrid_base))
        (Variables|/Game/Blueprint/Grid/GridBase.GridBase_C|SetUsed _asgrid_base true)))
    (:CastFailed
      (if (not (Variables|Default|Getfloor))
        (bind _asremovable_actor (Utilities|Casting|CastToRemovableActor OtherActor)
          (:then
            (if (not (Variables|RemovableActor_C|Getused? _asremovable_actor))
              (Variables|RemovableActor_C|Setused? _asremovable_actor true)))
          (:CastFailed
            (Actor|DestroyActor)))))))

(event OnComponentEndOverlap(Box)
  (params (OverlappedComponent :type Primitive%20Component%20Object%20Reference) (OtherActor :type Actor%20Object%20Reference) (OtherComp :type Primitive%20Component%20Object%20Reference) (OtherBodyIndex :type Integer))
  (bind _asgrid_base (Utilities|Casting|CastToGridBase OtherActor)
    (:then
      (if (Variables|/Game/Blueprint/Grid/GridBase.GridBase_C|GetUsed _asgrid_base)
        (Variables|/Game/Blueprint/Grid/GridBase.GridBase_C|SetUsed _asgrid_base false)))
    (:CastFailed
      (if (not (Variables|Default|Getfloor))
        (bind _asremovable_actor (Utilities|Casting|CastToRemovableActor OtherActor))
        (if (Variables|RemovableActor_C|Getused? _asremovable_actor)
          (Variables|RemovableActor_C|Setused? _asremovable_actor false))))))

(event EventBeginPlay
  (bind _returnvalue (Transformation|GetActorRotation))
  (bind _staticmesh (Variables|Default|GetStaticMesh))
  (bind _buttonrotate (Variables|Default|GetButtonRotate))
  (Transformation|SetActorRotation (Math|Rotator|MakeRotator (.roll _returnvalue) (.pitch _returnvalue) (+ (.yaw _returnvalue) 9e+01)))
  (Rendering|SetVisibility (Variables|Default|Gettext) false false)
  (bind _asbp_label_widget (Utilities|Casting|CastToBp_LabelWidget (UserInterface|GetUserWidgetObject (Variables|Default|Gettext))))
  (Variables|/Game/Widget/Bp_LabelWidget.Bp_LabelWidget_C|SetFurnitureReference _asbp_label_widget self)
  (Variables|Default|SetMaterialReference (Rendering|Material|GetMaterial (Variables|Default|GetStaticMesh) 0))
  (CallFunction|PlaceObjectOpacity)
  (Variables|Default|SetStaticRef _staticmesh)
  (Variables|Default|SetSelfStaticMesh (Variables|/Script/Engine.StaticMeshComponent|GetStaticMesh _staticmesh))
  (Rendering|SetVisibility _buttonrotate false false)
  (Variables|/Game/Widget/Bp_buttonRotate.Bp_buttonRotate_C|SetFurnitureReference (.AsBp%20Button%20Rotate (Utilities|Casting|CastToBp_buttonRotate (UserInterface|GetUserWidgetObject _buttonrotate))) self))

(event EventTick
  (params (DeltaSeconds :type Float%20%28single-precision%29))
  (Utilities|FlowControl|Sequence
    (:then_1
      (Utilities|IsValid (Variables|Default|GetMeshComp)
        (:Is%20Valid
          (Transformation|SetWorldTransform (Variables|Default|GetMeshComp) (Transformation|GetActorTransform) false true))))))

(fn ConstructionScript)

(fn MarkedRed
  (Rendering|Material|SetVectorParameterValueonMaterials (Variables|Default|GetStaticMesh) "color" "1.000000,0.000000,0.000000"))

(fn MarkedBlue
  (Rendering|Material|SetVectorParameterValueonMaterials (Variables|Default|GetStaticMesh) "color" "0.000000,0.000000,1.000000"))

(fn PlaceObjectOpacity
  (Rendering|Material|SetScalarParameterValueonMaterials (Variables|Default|GetStaticMesh) "opacity" (select (Variables|Default|Getplaced?) 1.0 0.2)))

(fn Select
  (bind _returnvalue (AddComponent|AddStaticMeshComponent true (Transformation|GetWorldTransform (Variables|Default|GetStaticRef))))
  (bind _output_get (Variables|Default|SetMeshComp _returnvalue))
  (Components|StaticMesh|SetStaticMesh _output_get (Variables|Default|GetSelfStaticMesh))
  (bind _returnvalue_2 (Rendering|Material|CreateDynamicMaterialInstance _output_get 0 "/Game/Material/M_outline_Inst.M_outline_Inst" "None" :!class /Script/Engine.PrimitiveComponent))
  (Rendering|Material|SetVectorParameterValue _returnvalue_2 "color" "(R=1.000000,G=0.896815,B=0.000000,A=1.000000)" :!class /Script/Engine.MaterialInstanceDynamic)
  (Rendering|Material|SetScalarParameterValue _returnvalue_2 "scale" 5.0 :!class /Script/Engine.MaterialInstanceDynamic)
  (if (not (Variables|Default|Getfloor))
    (Rendering|SetVisibility (Variables|Default|GetButtonRotate) true false)))

(fn Deselect
  (bind _meshcomp (Variables|Default|GetMeshComp))
  (Utilities|IsValid _meshcomp
    (:Is%20Valid
      (Components|DestroyComponent _meshcomp)
      (Rendering|SetVisibility (Variables|Default|GetButtonRotate) false false))))

(fn RotateLeft
  (bind _returnvalue (Transformation|GetActorRotation))
  (Transformation|AddActorLocalRotation (Math|Rotator|MakeRotator (.roll _returnvalue) (.pitch _returnvalue) -9e+01) false false))

(fn RotateRight
  (bind _returnvalue (Transformation|GetActorRotation))
  (Transformation|AddActorLocalRotation (Math|Rotator|MakeRotator (.roll _returnvalue) (.pitch _returnvalue) 9e+01) false false))