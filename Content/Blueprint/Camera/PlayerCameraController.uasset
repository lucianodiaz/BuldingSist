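; Player controller for a grid-based furniture builder that also moves and zooms the CameraPlayer pawn.
; A looping timer traces under the mouse to highlight GridBase cells by occupancy, spawn the chosen class on grids, floors or walls, or toggle RemovableActor selection.
; The selection menu receives the controller, and SetFurnitureClass sets what spawns.
; Input actions rotate, delete or open a color wheel for the selection, and toggle its label or all labels.
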(event Custom|TraceObjects
  (bind (_worldlocation _worlddirection) (Game|Player|ConvertMouseLocationToWorldSpace))
  (bind _classfurnituretospawn (Variables|Default|GetClassFurnitureToSpawn))
  (bind _returnvalue (!= _classfurnituretospawn 0))
  (bind (_outhit _returnvalue_2) (Collision|LineTraceByChannel _worldlocation (+ _worldlocation (* _worlddirection 5e+03)) "TraceTypeQuery1" false (Utilities|Array|MakeArray (Game|Player|GetPlayerPawn 0)) "None" true "(R=1.000000,G=0.000000,B=0.000000,A=1.000000)" "(R=0.000000,G=1.000000,B=0.000000,A=1.000000)" 1.0))
  (if _returnvalue_2
    ;[1 1 1] make all grid invisibles
    (bind _outactors (Actor|GetAllActorsOfClass "/Game/Blueprint/Grid/GridBase.GridBase_C"))
    (for _array_element _outactors
      (Default|DesactivePlane _array_element))
    ;[1 1 1] mark visible grid below mouse
    (bind _asgrid_base (Utilities|Casting|CastToGridBase (.HitActor (Collision|BreakHitResult _outhit)))
      (:then
        (Default|ActivePlane _asgrid_base)
        (if (Math|Boolean|Equal(Boolean) (Variables|/Game/Blueprint/Grid/GridBase.GridBase_C|GetUsed _asgrid_base) true)
          ;[1 1 1] Red
          (Default|MakeRedPosition _asgrid_base)
          (else
            ;[1 1 1] blue
            (Default|MakeBluePosition _asgrid_base)
            ;[1 1 1] spawn furniture
            (if (and (Variables|Default|GetActionPressed) (Math|Boolean|Equal(Boolean) (Variables|/Game/Blueprint/Grid/GridBase.GridBase_C|GetUsed _asgrid_base) false))
              (if (!= (Variables|Default|GetClassFurnitureToSpawn) 0)
                (bind _returnvalue_3 (Game|SpawnActorfromClass (Variables|Default|GetClassFurnitureToSpawn) (Math|Transform|MakeTransform (.location (Transformation|GetActorTransform _asgrid_base)) (.rotation (Transformation|GetActorTransform _asgrid_base))) "Undefined" 0 0))
                (if (or (Variables|/Game/Blueprint/furniture/RemovableActor.RemovableActor_C|Getfloor _returnvalue_3) (Variables|/Game/Blueprint/furniture/RemovableActor.RemovableActor_C|Getwall? _returnvalue_3))
                  (Variables|/Game/Blueprint/Grid/GridBase.GridBase_C|SetUsed _asgrid_base true)
                  (else
                    (Variables|Default|SetActionPressed false)
                    (Variables|/Game/Blueprint/Grid/GridBase.GridBase_C|SetUsed _asgrid_base true))))))))
      (:CastFailed
        (bind _asremovable_actor (Utilities|Casting|CastToRemovableActor (.HitActor (Collision|BreakHitResult _outhit))))
        ;[1 1 1] I ask if is it floor and if used and is action pressed (left button mouse)
        (if (Math|Boolean|ANDBoolean (Variables|/Game/Blueprint/furniture/RemovableActor.RemovableActor_C|Getfloor _asremovable_actor) (Math|Boolean|NotEqual(Boolean) (Variables|/Game/Blueprint/furniture/RemovableActor.RemovableActor_C|Getused? _asremovable_actor) true) (Variables|Default|GetActionPressed))
          ;[1 1 1] in floor is avalible spawn another furniture
          (if (Math|Boolean|ANDBoolean _returnvalue (!= _classfurnituretospawn "/Game/Blueprint/furniture/Floor.Floor_C") (!= _classfurnituretospawn "/Game/Blueprint/furniture/Panel.Panel_C"))
            ;[1 1 1] spawn above the floor
            (Game|SpawnActorfromClass (Variables|Default|GetClassFurnitureToSpawn) (Math|Transform|MakeTransform (.location (Transformation|GetActorTransform _asremovable_actor)) (.rotation (Transformation|GetActorTransform _asremovable_actor))) "Undefined" 0 0)
            (Variables|Default|SetActionPressed false)
            (Variables|/Game/Blueprint/furniture/RemovableActor.RemovableActor_C|Setused? _asremovable_actor true)
            (else
              ;[1 1 1] mark selected furniture/ floor
              (if (and (Math|Boolean|NotEqual(Boolean) _returnvalue true) (Variables|Default|GetActionPressed))
                (Utilities|IsValid (Variables|Default|GetFurnitureReference)
                  (:Is%20Valid
                    (if (== (Variables|Default|GetFurnitureReference) _asremovable_actor)
                      (Default|Deselect (Variables|Default|GetFurnitureReference))
                      (Variables|Default|SetFurnitureReference 0)
                      (else
                        (Default|Deselect (Variables|Default|GetFurnitureReference))
                        (bind _output_get (Variables|Default|SetFurnitureReference _asremovable_actor :!label _label))
                        (Default|Select _output_get))))
                  (:Is%20Not%20Valid
                    (goto _label)))
                (Variables|Default|SetActionPressed false))))
          (elif (Math|Boolean|ANDBoolean (Variables|/Game/Blueprint/furniture/RemovableActor.RemovableActor_C|Getwall? _asremovable_actor) (Math|Boolean|NotEqual(Boolean) (Variables|/Game/Blueprint/furniture/RemovableActor.RemovableActor_C|Getused? _asremovable_actor) true) (Variables|Default|GetActionPressed))
            (if (== (Variables|Default|GetClassFurnitureToSpawn) "/Game/Blueprint/furniture/Panel.Panel_C")
              (Game|SpawnActorfromClass (Variables|Default|GetClassFurnitureToSpawn) (Math|Transform|MakeTransform (.location (Transformation|GetWorldTransform (Variables|/Game/Blueprint/furniture/Wall.Wall_C|Getpoint (.AsWall (Utilities|Casting|CastToWall _asremovable_actor))))) (.rotation (Transformation|GetWorldTransform (Variables|/Game/Blueprint/furniture/Wall.Wall_C|Getpoint (.AsWall (Utilities|Casting|CastToWall _asremovable_actor))))) "1,1,1") "Undefined" 0 0)
              (Variables|Default|SetActionPressed false)
              (Variables|/Game/Blueprint/furniture/RemovableActor.RemovableActor_C|Setused? _asremovable_actor true)
              (else
                (if (Variables|Default|GetActionPressed) :!label _label_2
                  ;[1 1 1] Mark/ desmark selected furniture
                  (Utilities|IsValid (Variables|Default|GetFurnitureReference)
                    (:Is%20Valid
                      (if (== (Variables|Default|GetFurnitureReference) _asremovable_actor)
                        (Default|Deselect (Variables|Default|GetFurnitureReference))
                        (Variables|Default|SetFurnitureReference 0)
                        (else
                          (Default|Deselect (Variables|Default|GetFurnitureReference))
                          (bind _output_get_2 (Variables|Default|SetFurnitureReference _asremovable_actor :!label _label_3))
                          (Default|Select _output_get_2))))
                    (:Is%20Not%20Valid
                      (goto _label_3)))
                  (Variables|Default|SetActionPressed false))))
            (else
              (goto _label_2))))))))

(event Custom|OpenMenu
  ;[1 1 1] Open Menu Selection objects
  (Utilities|FlowControl|FlipFlop
    (:A
      (Utilities|FlowControl|Sequence
        (:then_0
          (Utilities|IsValid (Variables|Default|GetFurnitureReference)
            (:Is%20Valid
              (Default|Deselect (Variables|Default|GetFurnitureReference)))))
        (:then_1
          (Variables|Default|SetFurnitureReference 0)
          (bind _returnvalue (UserInterface|CreateWidget "/Game/Widget/Bp_MenuSelection.Bp_MenuSelection_C" (Game|GetPlayerController 0)))
          (Variables|Default|SetMenuFurnitureReference _returnvalue)
          (UserInterface|Viewport|AddtoViewport _returnvalue 0)
          (Input|SetInputModeGameandUI (Game|GetPlayerController 0) _returnvalue "DoNotLock" false)
          (Default|SetPlayerController _returnvalue self))))
    (:B
      (Utilities|IsValid (Variables|Default|GetMenuFurnitureReference)
        (:Is%20Valid
          (Widget|RemovefromParent (Variables|Default|GetMenuFurnitureReference)))))))

(event Custom|deleteFurniture
  ;[1 1 1] delete furniture
  (Utilities|IsValid (Variables|Default|GetFurnitureReference)
    (:Is%20Valid
      (Actor|DestroyActor (Variables|Default|GetFurnitureReference))
      (Variables|Default|SetFurnitureReference 0))))

(event Custom|changeColor
  ;[1 1 1] Change color
  (Utilities|FlowControl|FlipFlop
    (:A
      (Utilities|IsValid (Variables|Default|GetFurnitureReference)
        (:Is%20Valid
          (bind _returnvalue (UserInterface|CreateWidget "/Game/Widget/BP_WheelColor.BP_WheelColor_C"))
          (UserInterface|Viewport|AddtoViewport _returnvalue 0)
          (Class|PlayerController|SetMouseLocation (Math|Float|Truncate (/ (* (Class|WidgetLayoutLibrary|GetViewportScale) (.X (Math|Vector2D|BreakVector2D (Class|CanvasPanelSlot|GetSize (Class|WidgetLayoutLibrary|SlotasCanvasSlot (Variables|/Game/Widget/BP_WheelColor.BP_WheelColor_C|GetCanvasPanel_1 _returnvalue)))))) 2.0)) (Math|Float|Truncate (/ (* (.Y (Math|Vector2D|BreakVector2D (Class|CanvasPanelSlot|GetSize (Class|WidgetLayoutLibrary|SlotasCanvasSlot (Variables|/Game/Widget/BP_WheelColor.BP_WheelColor_C|GetCanvasPanel_1 _returnvalue))))) (Class|WidgetLayoutLibrary|GetViewportScale)) 2.0))))))
    (:B
      (bind _foundwidgets (Widget|GetAllWidgetsOfClass "/Game/Widget/BP_WheelColor.BP_WheelColor_C" true))
      (for _array_element _foundwidgets
        (Widget|RemovefromParent _array_element)))))

(event EventBeginPlay
  ;[1 1 1] Begin play
  (bind _ascamera_player (Utilities|Casting|CastToCameraPlayer (Pawn|GetControlledPawn)))
  (Variables|Default|SetCamRef _ascamera_player)
  (Variables|Default|SetbShowMouseCursor true)
  (Utilities|Time|SetTimerbyFunctionName 0 "TraceObjects" 0.05 true)
  (bind _returnvalue (Game|GetCurrentLevelName true))
  (if (Utilities|Enum|Equal(Enum) _returnvalue "ProofMap")
    (bind _returnvalue_2 (UserInterface|CreateWidget "/Game/Widget/BP_Options.BP_Options_C" 0 self))
    (UserInterface|Viewport|AddtoViewport _returnvalue_2 0)))

(event EventTick
  (params (DeltaSeconds :type Float%20%28single-precision%29)))

(event Input|ActionEvents|InputActionPressed
  (params (Key :type Key%20Structure :default "None"))
  ;[1 1 1] Action Pressed
  (:Pressed
    (Variables|Default|SetActionPressed true))
  (:Released
    (Variables|Default|SetActionPressed false)
    (Variables|Default|SetClassFurnitureToSpawn 0)))

(event Input|ActionEvents|InputActionRotateLeft
  (params (Key :type Key%20Structure :default "None"))
  (bind _furniturereference (Variables|Default|GetFurnitureReference))
  ;[1 1 1] Rotate left furnitures
  (:Pressed
    (Utilities|IsValid _furniturereference
      (:Is%20Valid
        (Default|RotateLeft _furniturereference)))))

(event Input|ActionEvents|InputActionRotateRight
  (params (Key :type Key%20Structure :default "None"))
  (bind _furniturereference (Variables|Default|GetFurnitureReference))
  ;[1 1 1] rotate right furniture
  (:Pressed
    (Utilities|IsValid _furniturereference
      (:Is%20Valid
        (Default|RotateRight _furniturereference)))))

(event Input|ActionEvents|InputActionDeleteFurniture
  (params (Key :type Key%20Structure :default "None"))
  ;[1 1 1] delete furniture
  (:Pressed
    (Utilities|IsValid (Variables|Default|GetFurnitureReference)
      (:Is%20Valid
        (Actor|DestroyActor (Variables|Default|GetFurnitureReference))
        (Variables|Default|SetFurnitureReference 0)))))

(event Input|ActionEvents|InputActionOpenMenu
  (params (Key :type Key%20Structure :default "None"))
  ;[1 1 1] Open Menu Selection objects
  (:Pressed
    (Utilities|FlowControl|FlipFlop
      (:A
        (Utilities|FlowControl|Sequence
          (:then_0
            (Utilities|IsValid (Variables|Default|GetFurnitureReference)
              (:Is%20Valid
                (Default|Deselect (Variables|Default|GetFurnitureReference)))))
          (:then_1
            (Variables|Default|SetFurnitureReference 0)
            (bind _returnvalue (UserInterface|CreateWidget "/Game/Widget/Bp_MenuSelection.Bp_MenuSelection_C" (Game|GetPlayerController 0)))
            (Variables|Default|SetMenuFurnitureReference _returnvalue)
            (UserInterface|Viewport|AddtoViewport _returnvalue 0)
            (Input|SetInputModeGameandUI (Game|GetPlayerController 0) _returnvalue "DoNotLock" false)
            (Default|SetPlayerController _returnvalue self))))
      (:B
        (Utilities|IsValid (Variables|Default|GetMenuFurnitureReference)
          (:Is%20Valid
            (Widget|RemovefromParent (Variables|Default|GetMenuFurnitureReference))))))))

(event Input|ActionEvents|InputActionShowLabel
  (params (Key :type Key%20Structure :default "None"))
  (bind _furniturereference (Variables|Default|GetFurnitureReference))
  (bind _furniturereference_2 (Variables|Default|GetFurnitureReference))
  (bind _text (Variables|/Game/Blueprint/furniture/RemovableActor.RemovableActor_C|Gettext _furniturereference_2))
  ;[1 1 1] Show labels selected furnitures
  (:Pressed
    (Utilities|FlowControl|FlipFlop
      (:A
        (Utilities|IsValid _furniturereference_2
          (:Is%20Valid
            (if (and (Math|Boolean|NotEqual(Boolean) (Variables|/Game/Blueprint/furniture/RemovableActor.RemovableActor_C|Getfloor _furniturereference_2) true) (Math|Boolean|NotEqual(Boolean) (Variables|/Game/Blueprint/furniture/RemovableActor.RemovableActor_C|Getwall? _furniturereference_2) true))
              (Default|SetText (.AsBp%20Label%20Widget (Utilities|Casting|CastToBp_LabelWidget (UserInterface|GetUserWidgetObject _text))) (Utilities|Text|ToText(String) (Variables|/Game/Blueprint/furniture/RemovableActor.RemovableActor_C|GetTitleLabel _furniturereference_2)) (Utilities|Text|ToText(String) (Variables|/Game/Blueprint/furniture/RemovableActor.RemovableActor_C|GettextLabel _furniturereference_2)))
              (Rendering|SetVisibility _text true false)))))
      (:B
        (Utilities|IsValid _furniturereference
          (:Is%20Valid
            (Rendering|SetVisibility (Variables|/Game/Blueprint/furniture/RemovableActor.RemovableActor_C|Gettext _furniturereference) false false)))))))

(event Input|ActionEvents|InputActionShowAllLabel
  (params (Key :type Key%20Structure :default "None"))
  ;[1 1 1] show all labels
  (:Pressed
    (Utilities|FlowControl|FlipFlop
      (:A
        (bind _outactors (Actor|GetAllActorsOfClass "/Game/Blueprint/furniture/RemovableActor.RemovableActor_C"))
        (for _array_element _outactors
          (if (and (Math|Boolean|NotEqual(Boolean) (Variables|/Game/Blueprint/furniture/RemovableActor.RemovableActor_C|Getfloor _array_element) true) (Math|Boolean|NotEqual(Boolean) (Variables|/Game/Blueprint/furniture/RemovableActor.RemovableActor_C|Getwall? _array_element) true))
            (Default|SetText (.AsBp%20Label%20Widget (Utilities|Casting|CastToBp_LabelWidget (UserInterface|GetUserWidgetObject (Variables|/Game/Blueprint/furniture/RemovableActor.RemovableActor_C|Gettext _array_element)))) (Utilities|Text|ToText(String) (Variables|/Game/Blueprint/furniture/RemovableActor.RemovableActor_C|GetTitleLabel _array_element)) (Utilities|Text|ToText(String) (Variables|/Game/Blueprint/furniture/RemovableActor.RemovableActor_C|GettextLabel _array_element)))
            (Rendering|SetVisibility (Variables|/Game/Blueprint/furniture/RemovableActor.RemovableActor_C|Gettext _array_element) true false))))
      (:B
        (bind _outactors_2 (Actor|GetAllActorsOfClass "/Game/Blueprint/furniture/RemovableActor.RemovableActor_C"))
        (for _array_element_2 _outactors_2
          (Rendering|SetVisibility (Variables|/Game/Blueprint/furniture/RemovableActor.RemovableActor_C|Gettext _array_element_2) false false))))))

(event Input|ActionEvents|InputActionChangeColor
  (params (Key :type Key%20Structure :default "None"))
  ;[1 1 1] Change color
  (:Pressed
    (Utilities|FlowControl|FlipFlop
      (:A
        (Utilities|IsValid (Variables|Default|GetFurnitureReference)
          (:Is%20Valid
            (bind _returnvalue (UserInterface|CreateWidget "/Game/Widget/BP_WheelColor.BP_WheelColor_C"))
            (UserInterface|Viewport|AddtoViewport _returnvalue 0)
            (Class|PlayerController|SetMouseLocation (Math|Float|Truncate (/ (* (Class|WidgetLayoutLibrary|GetViewportScale) (.X (Math|Vector2D|BreakVector2D (Class|CanvasPanelSlot|GetSize (Class|WidgetLayoutLibrary|SlotasCanvasSlot (Variables|/Game/Widget/BP_WheelColor.BP_WheelColor_C|GetCanvasPanel_1 _returnvalue)))))) 2.0)) (Math|Float|Truncate (/ (* (.Y (Math|Vector2D|BreakVector2D (Class|CanvasPanelSlot|GetSize (Class|WidgetLayoutLibrary|SlotasCanvasSlot (Variables|/Game/Widget/BP_WheelColor.BP_WheelColor_C|GetCanvasPanel_1 _returnvalue))))) (Class|WidgetLayoutLibrary|GetViewportScale)) 2.0))))))
      (:B
        (bind _foundwidgets (Widget|GetAllWidgetsOfClass "/Game/Widget/BP_WheelColor.BP_WheelColor_C" true))
        (for _array_element _foundwidgets
          (Widget|RemovefromParent _array_element))))))

(event Input|ActionEvents|InputActionZoomIn
  (params (Key :type Key%20Structure :default "None"))
  (bind _camref (Variables|Default|GetCamRef))
  (bind _springarm (Variables|/Game/Blueprint/Camera/CameraPlayer.CameraPlayer_C|GetSpringArm _camref))
  ;[1 1 1] Zoom in zoom out
  (:Pressed
    (Variables|/Script/Engine.SpringArmComponent|SetTargetArmLength _springarm (Math|Float|Clamp(Float) (Math|Interpolation|FInterpTo (Variables|/Script/Engine.SpringArmComponent|GetTargetArmLength _springarm) (- (Variables|/Script/Engine.SpringArmComponent|GetTargetArmLength _springarm) 1e+02) 1.0 1.0) 1e+01 8e+02))))

(event Input|ActionEvents|InputActionZoomOut
  (params (Key :type Key%20Structure :default "None"))
  (bind _camref (Variables|Default|GetCamRef))
  (bind _springarm (Variables|/Game/Blueprint/Camera/CameraPlayer.CameraPlayer_C|GetSpringArm _camref))
  ;[1 1 1] Zoom in zoom out
  (:Pressed
    (Variables|/Script/Engine.SpringArmComponent|SetTargetArmLength _springarm (Math|Float|Clamp(Float) (Math|Interpolation|FInterpTo (Variables|/Script/Engine.SpringArmComponent|GetTargetArmLength _springarm) (+ (Variables|/Script/Engine.SpringArmComponent|GetTargetArmLength _springarm) 1e+02) 1.0 1.0) 1e+01 8e+02))))

(event Input|AxisEvents|InputAxisright
  (params (AxisValue :type Float%20%28single-precision%29))
  (bind _camref (Variables|Default|GetCamRef))
  ;[1 1 1] Move camera right left forward backward
  (Class|PawnMovementComponent|AddInputVector (Variables|/Game/Blueprint/Camera/CameraPlayer.CameraPlayer_C|GetFloatingPawnMovement _camref) (* (Transformation|GetActorRightVector _camref) AxisValue) false))

(event Input|AxisEvents|InputAxisforward
  (params (AxisValue :type Float%20%28single-precision%29))
  (bind _camref (Variables|Default|GetCamRef))
  ;[1 1 1] Move camera right left forward backward
  (Class|PawnMovementComponent|AddInputVector (Variables|/Game/Blueprint/Camera/CameraPlayer.CameraPlayer_C|GetFloatingPawnMovement _camref) (* (Transformation|GetActorForwardVector _camref) AxisValue) false))

(fn ConstructionScript)

(fn SetFurnitureClass
  (params (Furniture :type Removable%20Actor%20Class%20Reference))
  (Variables|Default|SetClassFurnitureToSpawn Furniture))