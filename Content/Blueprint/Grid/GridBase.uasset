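; GridBase is a grid actor whose plane shows position state through color.
; BeginPlay creates a dynamic instance of M_Grid_base on the plane, and custom events set its color parameter to red or blue or toggle the plane's visibility.
; Tick reapplies red every frame while Used is true; blue and visibility changes are not triggered within this graph.
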(event Custom|DesactivePlane
  (Rendering|SetVisibility (Variables|Default|Getplane) false false))

(event Custom|ActivePlane
  (Rendering|SetVisibility (Variables|Default|Getplane) true false))

(event Custom|MakeRedPosition
  (Rendering|Material|SetVectorParameterValue (Variables|Default|GetMaterialRef) "color" "(R=1.000000,G=0.030943,B=0.000000,A=1.000000)" :!class /Script/Engine.MaterialInstanceDynamic))

(event Custom|MakeBluePosition
  (Rendering|Material|SetVectorParameterValue (Variables|Default|GetMaterialRef) "color" "(R=0.000000,G=0.638534,B=1.000000,A=1.000000)" :!class /Script/Engine.MaterialInstanceDynamic))

(event EventBeginPlay
  (bind _returnvalue (Rendering|Material|CreateDynamicMaterialInstance (Variables|Default|Getplane) 0 "/Game/Material/M_Grid_base.M_Grid_base" "None" :!class /Script/Engine.PrimitiveComponent))
  (Variables|Default|SetMaterialRef _returnvalue))

(event Collision|EventActorBeginOverlap
  (params (OtherActor :type Actor%20Object%20Reference)))

(event EventTick
  (params (DeltaSeconds :type Float%20%28single-precision%29))
  (if (Variables|Default|GetUsed)
    (CallFunction|MakeRedPosition)))

(fn ConstructionScript)