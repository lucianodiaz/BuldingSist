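; GridSetup is an actor that builds a flat grid of GridBase actors when play begins.
; Nested loops over GridX and GridY spawn one cell per step, spaced by GridSize and centered on the actor's location in world-aligned X and Y.
; Each spawned cell is stored in GridBaseArray.
; Spawning always succeeds, nudging cells clear of collisions where possible.
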(event EventBeginPlay
  (bind _grid_size (Variables|Default|GetGrid_size))
  (bind _grid_size_2 (Variables|Default|GetGrid_size))
  (bind _grid_size_3 (Variables|Default|GetGrid_size))
  (bind _returnvalue (/ _grid_size_2 2))
  (bind _returnvalue_2 (Math|Conversions|ToFloat(Integer) _returnvalue))
  (for _index (range 1 (Variables|Default|GetGrid_x))
    (for _index_2 (range 1 (Variables|Default|GetGrid_y))
      ;[1 1 1] Spawn go here
      (bind _returnvalue_3 (Game|SpawnActorfromClass "/Game/Blueprint/Grid/GridBase.GridBase_C" (Math|Transform|MakeTransform (+ (Transformation|GetActorLocation) (Math|Vector|MakeVector (- (Math|Conversions|ToFloat(Integer) (- (* _index _grid_size_3) (/ (* (Variables|Default|GetGrid_x) _grid_size) 2))) _returnvalue_2) (- (Math|Conversions|ToFloat(Integer) (- (* _index_2 _grid_size_3) (/ (* (Variables|Default|GetGrid_y) _grid_size) 2))) _returnvalue_2) 0.0))) "AdjustIfPossibleButAlwaysSpawn" 0 0))
      (Utilities|Array|Add (Variables|Default|GetGridBaseArray) _returnvalue_3))))

(event Collision|EventActorBeginOverlap
  (params (OtherActor :type Actor%20Object%20Reference)))

(event EventTick
  (params (DeltaSeconds :type Float%20%28single-precision%29)))

(fn ConstructionScript)